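; BP_ControlTable is a table with a hologram volume that displays miniature ships.
; On BeginPlay it spawns a BP_GenericShip at ChildAttachmentPoint, attaches it, scales its root down to one-tenth and assigns the first movement and weapon target actors found in the level.
; HologramCollisionMesh overlaps unhide any generic ship entering the volume and hide it on exit, so the mesh bounds the visible display.
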(event `self.ReceiveBeginPlay`
  (bind _childattachmentpoint (`self.ChildAttachmentPoint`))
  (bind _returnvalue (`|SpawnActorFromClass` "/Game/Blueprints/BP_GenericShip.BP_GenericShip_C" (`KismetMathLibrary.MakeTransform` (`SceneComponent.K2_GetComponentLocation` _childattachmentpoint) (`SceneComponent.K2_GetComponentRotation` _childattachmentpoint)) "Undefined" "OverrideRootScale" null null))
  (`self.K2_AttachToComponent` _returnvalue (`self.ChildAttachmentPoint`) "None" "KeepWorld" "KeepWorld" "KeepWorld" false)
  (`SceneComponent.SetRelativeScale3D` (`/Game/Blueprints/BP_GenericShip.ShipRootPoint` _returnvalue) (0.1 0.1 0.1))
  (bind _outactors (`GameplayStatics.GetAllActorsOfClass` "/Game/Blueprints/BP_ShipMovementTarget.BP_ShipMovementTarget_C"))
  (set `/Game/Blueprints/BP_GenericShip.ship_movement_target` (`|GetArrayItem` _outactors) _returnvalue)
  (bind _outactors_2 (`GameplayStatics.GetAllActorsOfClass` "/Game/Blueprints/BP_ShipWeaponTarget.BP_ShipWeaponTarget_C"))
  (set `/Game/Blueprints/BP_GenericShip.ship_weapons_target` (`|GetArrayItem` _outactors_2) _returnvalue))

(event `self.HologramCollisionMesh.OnComponentEndOverlap`
  (params (OverlappedComponent :type "PrimitiveComponent Object Reference") (OtherActor :type "Actor Object Reference") (OtherComp :type "PrimitiveComponent Object Reference") (OtherBodyIndex :type Integer))
  (bind _asbp_generic_ship (cast `/Game/Blueprints/BP_GenericShip` OtherActor))
  (`self.SetActorHiddenInGame` _asbp_generic_ship true))

(event `self.HologramCollisionMesh.OnComponentBeginOverlap`
  (params (OverlappedComponent :type "PrimitiveComponent Object Reference") (OtherActor :type "Actor Object Reference") (OtherComp :type "PrimitiveComponent Object Reference") (OtherBodyIndex :type Integer) (bFromSweep :type Boolean) (SweepResult :type "HitResult Structure (by ref)"))
  (bind _asbp_generic_ship (cast `/Game/Blueprints/BP_GenericShip` OtherActor))
  (`self.SetActorHiddenInGame` _asbp_generic_ship false))

(fn `UserConstructionScript`)