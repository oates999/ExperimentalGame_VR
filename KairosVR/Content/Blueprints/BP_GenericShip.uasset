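; BP_GenericShip is a ship with simple hand-written physics that homes toward a movement target actor.
; Each Tick integrates velocity and location, then adds force along a yaw-aimed MovementArrow into a persistent, capped acceleration; velocity is also capped.
; Space yaws the ship root toward a weapons target and draws a short debug line trace without applying hits.
; C toggles slow-motion time dilation.
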(event `Key|C`
  (params (Key :type "Key Structure"))
  (:`Pressed`
    (if (== (`GameplayStatics.GetGlobalTimeDilation`) 1.0)
      (`GameplayStatics.SetGlobalTimeDilation` 0.1)
      (else
        (`GameplayStatics.SetGlobalTimeDilation` 1.0)))))

(event `Key|SpaceBar`
  (params (Key :type "Key Structure"))
  (:`Pressed`
    (`self.Fire Weapons Towards Location` (`self.K2_GetActorLocation` (`self.ship_weapons_target`)))))

(event `self.ReceiveTick`
  (params (DeltaSeconds :type "Float (single-precision)"))
  (`|ExecutionSequence`
    (:`then_0`
      ;[1 1 1] Physics Updates
      (`self.Update Velocity` DeltaSeconds)
      (`self.Update Location` DeltaSeconds))
    (:`then_1`
      (`self.Add Force Towards Location` (`self.K2_GetActorLocation` (`self.ship_movement_target`)) 1000.0))))

(event `Add Force Towards Location`
  (params (location :type "Vector Structure") (force :type "Float (double-precision)"))
  (bind _movementarrow (`self.MovementArrow`))
  (bind (_returnvalue_roll _returnvalue_pitch) (`KismetMathLibrary.BreakRotator` (`SceneComponent.K2_GetComponentRotation` _movementarrow)))
  (bind (_returnvalue_roll_2 _returnvalue_pitch_2 _returnvalue_yaw) (`KismetMathLibrary.BreakRotator` (`KismetMathLibrary.FindLookAtRotation` (`SceneComponent.K2_GetComponentLocation` _movementarrow) location)))
  (`SceneComponent.K2_SetWorldRotation` _movementarrow (`KismetMathLibrary.MakeRotator` _returnvalue_roll _returnvalue_pitch _returnvalue_yaw) false false)
  (`self.Add Force` (* (`SceneComponent.GetForwardVector` (`self.MovementArrow`)) force)))

(event `Fire Weapons Towards Location`
  (params (location :type "Vector Structure"))
  (bind _shiprootpoint (`self.ShipRootPoint`))
  (bind _shiprootpoint_2 (`self.ShipRootPoint`))
  (bind (_returnvalue_roll _returnvalue_pitch) (`KismetMathLibrary.BreakRotator` (`SceneComponent.K2_GetComponentRotation` _shiprootpoint_2)))
  (bind _returnvalue (`SceneComponent.K2_GetComponentLocation` _shiprootpoint))
  (bind (_returnvalue_roll_2 _returnvalue_pitch_2 _returnvalue_yaw) (`KismetMathLibrary.BreakRotator` (`KismetMathLibrary.FindLookAtRotation` _returnvalue location)))
  (`SceneComponent.K2_SetWorldRotation` _shiprootpoint_2 (`KismetMathLibrary.MakeRotator` _returnvalue_roll _returnvalue_pitch _returnvalue_yaw) false false)
  (`KismetSystemLibrary.LineTraceSingle` :`Start` _returnvalue :`End` (+ _returnvalue (* (`SceneComponent.GetForwardVector` _shiprootpoint) 100.0)) :`TraceChannel` "TraceTypeQuery1" :`DrawDebugType` "ForDuration" :`DrawTime` 1.0))

(fn `Add Force`
  (params (force :type "Vector Structure"))
  (bind _max_acceleration (`self.max_acceleration`))
  (bind _new_acceleration (`self.Get New Acceleration` (`self.mass`) (`self.acceleration`) force))
  (bind _returnvalue (`KismetMathLibrary.VSize` _new_acceleration))
  (if (<= _returnvalue _max_acceleration)
    (set `self.acceleration` _new_acceleration)
    (else
      (set `self.acceleration` (* _new_acceleration (/ _max_acceleration _returnvalue))))))

(fn `Update Location`
  (params (delta_seconds :type "Float (double-precision)"))
  (`SceneComponent.K2_SetRelativeLocation` (`self.ShipRootPoint`) (`self.Get New Location` delta_seconds (`SceneComponent.RelativeLocation` (`self.ShipRootPoint`)) (`self.velocity`)) false true))

(fn `Update Velocity`
  (params (delta_seconds :type "Float (double-precision)"))
  (bind _max_velocity (`self.max_velocity`))
  (bind _new_velocity (`self.Get New Velocity` delta_seconds (`self.velocity`) (`self.acceleration`)))
  (bind _returnvalue (`KismetMathLibrary.VSize` _new_velocity))
  (if (<= _returnvalue _max_velocity)
    (set `self.velocity` _new_velocity)
    (else
      (set `self.velocity` (* _new_velocity (/ _max_velocity _returnvalue))))))

(fn `UserConstructionScript`)