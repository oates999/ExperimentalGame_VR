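; Rail gun weapon Blueprint that fires repeated line traces toward a target actor passed to FireAtActor.
; Each shot randomizes BulletDirection yaw within BulletSpread, turns WeaponDirection toward the target, then traces along BulletDirection out to Range.
; A DoOnce and ResetFire timer pace shots by RateOfFire, repeating while IsFiring is set.
; Traces draw timed debug lines, and their hit results are unused.
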(event `ResetFire`
  (bind _returnvalue (`SceneComponent.K2_GetComponentLocation` (`self.weapon_direction`)))
  (bind _returnvalue_2 (/ (`self.bullet_spread`) 2.0))
  (`|ExecutionSequence`
    (:`then_0`
      (goto _label :!via `Reset`))
    (:`then_1`
      (if (`self.is_firing`)
        (`/Engine/EditorBlueprintResources/StandardMacros.DoOnce` false :!label _label
          (:`Completed`
            (`SceneComponent.K2_SetRelativeRotation` (`self.bullet_direction`) (`KismetMathLibrary.MakeRotator` 0.0 0.0 (`KismetMathLibrary.RandomFloatInRange` (* -1 _returnvalue_2) _returnvalue_2)) false false)
            (`SceneComponent.K2_SetWorldRotation` (`self.weapon_direction`) (`KismetMathLibrary.FindLookAtRotation` (`SceneComponent.K2_GetComponentLocation` (`self.weapon_direction`)) (`self.K2_GetActorLocation` (stale `Fire At Actor` actor))) false false)
            (`KismetSystemLibrary.LineTraceSingle` :`Start` _returnvalue :`End` (+ _returnvalue (* (`SceneComponent.GetForwardVector` (`self.bullet_direction`)) (`self.range`))) :`TraceChannel` "TraceTypeQuery1" :`DrawDebugType` "ForDuration" :`TraceColor` (struct :`R` 1.0) :`TraceHitColor` (`self.trace_color`) :`DrawTime` (* (`self.rate_of_fire`) 0.8))
            (`KismetSystemLibrary.K2_SetTimerDelegate` (delegate `ResetFire`) (`self.rate_of_fire`))))))))

(event `Fire At Actor`
  (params (actor :type "Actor Object Reference"))
  (goto _label))

(fn `UserConstructionScript`)