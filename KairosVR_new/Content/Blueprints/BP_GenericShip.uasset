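; Player ship for motion-controller play that registers with the MotionControllerPawn and chases a movement target.
; Tick drives custom force, acceleration and velocity integration with clamped maximums, using eased scaling by target distance to damp motion on approach.
; It spawns an attached minigun and railgun; F swaps the active one and the right trigger fires it at the weapons target.
; Either grip toggles slow-motion through global time dilation.
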(event `self.ReceiveBeginPlay`
  (`|ExecutionSequence`
    (:`then_0`
      (bind _asmotion_controller_pawn (cast `/Game/VirtualRealityBP/Blueprints/MotionControllerPawn` (`GameplayStatics.GetPlayerPawn` 0)))
      (set `/Game/VirtualRealityBP/Blueprints/MotionControllerPawn.player_ship` self _asmotion_controller_pawn))
    (:`then_1`
      ;[1 1 1] Weapon Spawning
      (`|ExecutionSequence`
        (:`then_0`
          (bind _returnvalue (`|SpawnActorFromClass` "/Game/Blueprints/BP_Weapon_Minigun.BP_Weapon_Minigun_C" (`SceneComponent.K2_GetComponentToWorld` (`self.WeaponsArrow`)) "Undefined" "OverrideRootScale" null null))
          (`self.K2_AttachToComponent` _returnvalue (`self.WeaponsArrow`) "None" "KeepWorld" "KeepWorld" "KeepWorld" false)
          (set `self.minigun` _returnvalue))
        (:`then_1`
          (bind _returnvalue_2 (`|SpawnActorFromClass` "/Game/Blueprints/BP_Weapon_RailGun.BP_Weapon_RailGun_C" (`SceneComponent.K2_GetComponentToWorld` (`self.WeaponsArrow`)) "Undefined" "OverrideRootScale" null null))
          (`self.K2_AttachToComponent` _returnvalue_2 (`self.WeaponsArrow`) "None" "KeepWorld" "KeepWorld" "KeepWorld" false)
          (set `self.railgun` _returnvalue_2))))))

(event `Key|MotionController_Left_Grip1`
  (params (Key :type "Key Structure"))
  (:`Pressed`
    (if (== (`GameplayStatics.GetGlobalTimeDilation`) 1.0) :!label _label
      (`GameplayStatics.SetGlobalTimeDilation` 0.1)
      (else
        (`GameplayStatics.SetGlobalTimeDilation` 1.0)))))

(event `Key|F`
  (params (Key :type "Key Structure"))
  (:`Pressed`
    (if (`KismetStringLibrary.EqualEqual_StrStr` (`self.current_weapon`) "minigun")
      (set `self.current_weapon` "railgun")
      (else
        (set `self.current_weapon` "minigun")))))

(event `Key|MotionController_Right_Grip1`
  (params (Key :type "Key Structure"))
  (:`Pressed`
    (goto _label)))

(event `Key|MotionController_Right_Trigger`
  (params (Key :type "Key Structure"))
  (:`Pressed`
    (`self.Fire Weapons` true))
  (:`Released`
    (`self.Fire Weapons` false)))

(event `self.ReceiveTick`
  (params (DeltaSeconds :type "Float (single-precision)"))
  (bind _result (`|EaseFunction` "CircularOut" (`KismetMathLibrary.FMin` (/ (`KismetMathLibrary.VSize` (- (`self.K2_GetActorLocation` (`self.ship_movement_target`)) (`SceneComponent.K2_GetComponentLocation` (`self.ShipRootPoint`)))) (`self.deceleration_distance`)) 1.0) (+ 0.5 0.0) (+ 1.2 0.0)))
  (`|ExecutionSequence`
    (:`then_0`
      ;[1 1 1] Physics Updates
      (set `self.velocity` (* (`self.velocity`) _result))
      (set `self.acceleration` (* (`self.acceleration`) _result))
      (`self.Update Velocity` DeltaSeconds)
      (`self.Update Location` DeltaSeconds))
    (:`then_1`
      (`self.Add Force Towards Location` (`self.K2_GetActorLocation` (`self.ship_movement_target`)) 1000.0))))

(event `Add Force Towards Location`
  (params (location :type "Vector Structure") (force :type "Float (double-precision)"))
  (bind _movementarrow (`self.MovementArrow`))
  (bind (_returnvalue_roll _returnvalue_pitch _returnvalue_yaw) (`KismetMathLibrary.BreakRotator` (`KismetMathLibrary.FindLookAtRotation` (`SceneComponent.K2_GetComponentLocation` _movementarrow) location)))
  (`SceneComponent.K2_SetWorldRotation` _movementarrow (`KismetMathLibrary.MakeRotator` _returnvalue_roll _returnvalue_pitch _returnvalue_yaw) false false)
  (`self.Add Force` (* (`SceneComponent.GetForwardVector` (`self.MovementArrow`)) force)))

(event `Fire Weapons`
  (params (`Start/Stop` :type Boolean))
  (`|ExecutionSequence`
    (:`then_0`
      (if (`KismetStringLibrary.EqualEqual_StrStr` (`self.current_weapon`) "minigun")
        (bind _output_get (set `/Game/Blueprints/BP_Weapon_Minigun.is_firing` `Start/Stop` (`self.minigun`)))
        (if _output_get
          (`/Game/Blueprints/BP_Weapon_Minigun.Fire At Actor` (`self.minigun`) (`self.ship_weapons_target`)))))
    (:`then_1`
      (if (`KismetStringLibrary.EqualEqual_StrStr` (`self.current_weapon`) "railgun")
        (set `/Game/Blueprints/BP_Weapon_RailGun.is_firing` `Start/Stop` (`self.railgun`))
        (if true
          (`/Game/Blueprints/BP_Weapon_RailGun.Fire At Actor` (`self.railgun`) (`self.ship_weapons_target`)))))))

(event `Update Active Weapon`
  (params (new_weapon :type String))
  (bind _output_get (set `self.current_weapon` new_weapon))
  (`StaticMeshComponent.SetStaticMesh` (`self.WeaponMesh`) (`BlueprintMapLibrary.Map_Find` (`self.weapon_models`) _output_get)))

(fn `Add Force`
  (params (force :type "Vector Structure"))
  (bind _max_acceleration (`self.max_acceleration`))
  (bind _new_acceleration (`self.Get New Acceleration` (`self.mass`) (`self.acceleration`) force))
  (bind _returnvalue (`KismetMathLibrary.VSize` _new_acceleration))
  (if (<= _returnvalue _max_acceleration)
    (set `self.acceleration` _new_acceleration)
    (else
      (set `self.acceleration` (* _new_acceleration (/ _max_acceleration _returnvalue))))))

(fn `Update Location`
  (params (delta_seconds :type "Float (double-precision)"))
  (`SceneComponent.K2_SetRelativeLocation` (`self.ShipRootPoint`) (`self.Get New Location` delta_seconds (`SceneComponent.RelativeLocation` (`self.ShipRootPoint`)) (`self.velocity`)) false true))

(fn `Update Velocity`
  (params (delta_seconds :type "Float (double-precision)"))
  (bind _max_velocity (`self.max_velocity`))
  (bind _new_velocity (`self.Get New Velocity` delta_seconds (`self.velocity`) (`self.acceleration`)))
  (bind _returnvalue (`KismetMathLibrary.VSize` _new_velocity))
  (if (<= _returnvalue _max_velocity)
    (set `self.velocity` _new_velocity)
    (else
      (set `self.velocity` (* _new_velocity (/ _max_velocity _returnvalue))))))

(fn `UserConstructionScript`)