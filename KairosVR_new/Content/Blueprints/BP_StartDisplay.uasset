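; BP_StartDisplay is a VR start prompt that pauses the game on BeginPlay by zeroing global time dilation and disabling the first BP_GenericShip's ability.
; Left and right motion controllers set flags on the Yes and No colliders respectively; end overlaps also set them true, so they latch.
; Tick restores time and the ability, then destroys the display once both are set.
; UpdateButtonDisplay handles text highlighting but is not called here.
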(event `self.ReceiveBeginPlay`
  (bind _outactors (`GameplayStatics.GetAllActorsOfClass` "/Game/Blueprints/BP_GenericShip.BP_GenericShip_C"))
  (set `/Game/Blueprints/BP_GenericShip.ability_available` false (`|GetArrayItem` _outactors))
  (`GameplayStatics.SetGlobalTimeDilation` 0.0))

(event `Update Button Display`
  (`|ExecutionSequence`
    (:`then_0`
      (if (`self.left_overlap`)
        (`TextRenderComponent.SetTextRenderColor` (`self.YesText`) (`self.highlight_color`))
        (else
          (`TextRenderComponent.SetTextRenderColor` (`self.YesText`) (`self.default_color`)))))
    (:`then_1`
      (if (`self.right_overlap`)
        (`TextRenderComponent.SetTextRenderColor` (`self.NoText`) (`self.highlight_color`))
        (else
          (`TextRenderComponent.SetTextRenderColor` (`self.NoText`) (`self.default_color`)))))))

(event `self.ReceiveTick`
  (params (DeltaSeconds :type "Float (single-precision)"))
  (if (and (`self.left_overlap`) (`self.right_overlap`))
    (bind _outactors (`GameplayStatics.GetAllActorsOfClass` "/Game/Blueprints/BP_GenericShip.BP_GenericShip_C"))
    (set `/Game/Blueprints/BP_GenericShip.ability_available` true (`|GetArrayItem` _outactors))
    (`GameplayStatics.SetGlobalTimeDilation` 1.0)
    (`self.K2_DestroyActor`)))

(event `self.YesCollision.OnComponentBeginOverlap`
  (params (OverlappedComponent :type "PrimitiveComponent Object Reference") (OtherActor :type "Actor Object Reference") (OtherComp :type "PrimitiveComponent Object Reference") (OtherBodyIndex :type Integer) (bFromSweep :type Boolean) (SweepResult :type "HitResult Structure (by ref)"))
  (bind _asbp_motion_controller (cast `/Game/VirtualRealityBP/Blueprints/BP_MotionController` OtherActor))
  (if (`|EnumEquality` (`/Game/VirtualRealityBP/Blueprints/BP_MotionController.Hand` _asbp_motion_controller) "Left")
    (set `self.left_overlap` true)))

(event `self.YesCollision.OnComponentEndOverlap`
  (params (OverlappedComponent :type "PrimitiveComponent Object Reference") (OtherActor :type "Actor Object Reference") (OtherComp :type "PrimitiveComponent Object Reference") (OtherBodyIndex :type Integer))
  (bind _asbp_motion_controller (cast `/Game/VirtualRealityBP/Blueprints/BP_MotionController` OtherActor))
  (if (`|EnumEquality` (`/Game/VirtualRealityBP/Blueprints/BP_MotionController.Hand` _asbp_motion_controller) "Left")
    (set `self.left_overlap` true)))

(event `self.NoCollision.OnComponentBeginOverlap`
  (params (OverlappedComponent :type "PrimitiveComponent Object Reference") (OtherActor :type "Actor Object Reference") (OtherComp :type "PrimitiveComponent Object Reference") (OtherBodyIndex :type Integer) (bFromSweep :type Boolean) (SweepResult :type "HitResult Structure (by ref)"))
  (bind _asbp_motion_controller (cast `/Game/VirtualRealityBP/Blueprints/BP_MotionController` OtherActor))
  (if (`|EnumEquality` (`/Game/VirtualRealityBP/Blueprints/BP_MotionController.Hand` _asbp_motion_controller) "Right")
    (set `self.right_overlap` true)))

(event `self.NoCollision.OnComponentEndOverlap`
  (params (OverlappedComponent :type "PrimitiveComponent Object Reference") (OtherActor :type "Actor Object Reference") (OtherComp :type "PrimitiveComponent Object Reference") (OtherBodyIndex :type Integer))
  (bind _asbp_motion_controller (cast `/Game/VirtualRealityBP/Blueprints/BP_MotionController` OtherActor))
  (if (`|EnumEquality` (`/Game/VirtualRealityBP/Blueprints/BP_MotionController.Hand` _asbp_motion_controller) "Right")
    (set `self.right_overlap` true)))

(fn `UserConstructionScript`)