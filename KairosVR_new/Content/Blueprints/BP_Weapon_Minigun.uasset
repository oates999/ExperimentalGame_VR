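; Minigun weapon Blueprint that fires bullets toward a target actor passed to FireAtActor.
; A DoOnce gate and a ResetFire timer pace shots at RateOfFire, repeating while IsFiring is true.
; Each shot randomizes spread, aims at the target and spawns BP_Bullet_Minigun with a lifespan derived from range and speed.
; A legacy line trace still runs per shot, but its result is unused.
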(event `ResetFire`
  (bind _weapon_root (`self.weapon_root`))
  (bind _returnvalue (`SceneComponent.K2_GetComponentLocation` (`self.weapon_direction`)))
  (bind _returnvalue_2 (/ (`self.bullet_spread`) 2.0))
  (bind _returnvalue_3 (/ (`self.bullet_spread`) 2.0))
  (bind _returnvalue_4 (/ (`self.bullet_spread`) 2.0))
  (`|ExecutionSequence`
    (:`then_0`
      (goto _label :!via `Reset`))
    (:`then_1`
      (if (`self.is_firing`)
        (`/Engine/EditorBlueprintResources/StandardMacros.DoOnce` false :!label _label
          (:`Completed`
            (`SceneComponent.K2_SetRelativeRotation` (`self.bullet_direction`) (`KismetMathLibrary.MakeRotator` (`KismetMathLibrary.RandomFloatInRange` (* -1 _returnvalue_3) _returnvalue_3) (`KismetMathLibrary.RandomFloatInRange` (* -1 _returnvalue_4) _returnvalue_4) (`KismetMathLibrary.RandomFloatInRange` (* -1 _returnvalue_2) _returnvalue_2)) false false)
            (`SceneComponent.K2_SetWorldRotation` (`self.weapon_direction`) (`KismetMathLibrary.FindLookAtRotation` (`SceneComponent.K2_GetComponentLocation` (`self.weapon_direction`)) (`self.K2_GetActorLocation` (stale `Fire At Actor` actor))) false false)
            (`|ExecutionSequence`
              (:`then_0`
                (`KismetSystemLibrary.K2_SetTimerDelegate` (delegate `ResetFire`) (`self.rate_of_fire`)))
              (:`then_1`
                ;[1 1 1] LineTrace (Legacy)
                (`KismetSystemLibrary.LineTraceSingle` :`Start` _returnvalue :`End` (+ _returnvalue (* (`SceneComponent.GetForwardVector` (`self.bullet_direction`)) (`self.range`))) :`TraceChannel` "TraceTypeQuery1" :`TraceColor` (struct :`R` 1.0) :`TraceHitColor` (`self.trace_color`) :`DrawTime` (* (`self.rate_of_fire`) 1.5)))
              (:`then_2`
                ;[1 1 1] Bullet Spawning
                (bind _returnvalue_5 (`|SpawnActorFromClass` "/Game/Blueprints/BP_Bullet_Minigun.BP_Bullet_Minigun_C" (`KismetMathLibrary.MakeTransform` (`SceneComponent.K2_GetComponentLocation` _weapon_root) (`SceneComponent.K2_GetComponentRotation` (`self.bullet_direction`)) (`SceneComponent.K2_GetComponentScale` _weapon_root)) "Undefined" "OverrideRootScale" null (* (`SceneComponent.GetForwardVector` (`self.bullet_direction`)) (`self.bullet_speed`)) null))
                (`self.SetLifeSpan` _returnvalue_5 (/ (`self.range`) (`self.bullet_speed`)))))))))))

(event `Fire At Actor`
  (params (actor :type "Actor Object Reference"))
  (goto _label))

(fn `UserConstructionScript`)