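; BP_ScoreDisplay shows a running score in the world through a text render component.
; On begin play it displays the current score in the base text color.
; UpdateScore adds the incoming value to the total, refreshes the text, and plays the ColorLerp timeline to blend the color between base and highlight.
; The timeline uses Play rather than PlayFromStart, so it does not rewind between updates.
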(event `self.ReceiveBeginPlay`
  (bind _scoretext (`self.ScoreText`))
  (`TextRenderComponent.K2_SetText` _scoretext (`KismetTextLibrary.Conv_IntToText` (`self.score`)))
  (`TextRenderComponent.SetTextRenderColor` _scoretext (`self.text_color`)))

(event `Update Score`
  (params (incoming_score :type Integer))
  (set `self.score` (+ incoming_score (`self.score`)))
  (`TextRenderComponent.K2_SetText` (`self.ScoreText`) (`KismetTextLibrary.Conv_IntToText` (`self.score`)))
  (bind (_direction _alpha) (`Timeline|Color Lerp`)
    (:`Update`
      (`TextRenderComponent.SetTextRenderColor` (`self.ScoreText`) (`KismetMathLibrary.Conv_LinearColorToColor` (`KismetMathLibrary.LinearColorLerp` (`KismetMathLibrary.Conv_ColorToLinearColor` (`self.text_color`)) (`KismetMathLibrary.Conv_ColorToLinearColor` (`self.highlight_color`)) _alpha))))))

(fn `UserConstructionScript`)