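; Ship interior actor that controls its wall and ceiling lighting, with standard and hazard color states.
; The construction script applies the brightness and standard color variables to eight wall lights and six ceiling lights.
; ChangetoHazard and ChangetoStandard events swap wall and ceiling colors at runtime, reapplying the same brightness in both states.
; Each light component is set individually, so the same setup is repeated across all three graphs.
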(event `Change to Hazard`
  (bind _ceiling_brightness (`self.ceiling_brightness`))
  (bind _wall_brightness (`self.wall_brightness`))
  (bind _returnvalue (`KismetMathLibrary.Conv_ColorToLinearColor` (`self.ceiling_hazard_color`)))
  (bind _returnvalue_2 (`KismetMathLibrary.Conv_ColorToLinearColor` (`self.wall_hazard_color`)))
  (`|ExecutionSequence`
    (:`then_0`
      (`LightComponent.SetIntensity` (`self.C1Light1`) _wall_brightness)
      (`LightComponent.SetIntensity` (`self.C1Light2`) _wall_brightness)
      (`LightComponent.SetIntensity` (`self.C2Light1`) _wall_brightness)
      (`LightComponent.SetIntensity` (`self.C2Light2`) _wall_brightness)
      (`LightComponent.SetIntensity` (`self.C3Light1`) _wall_brightness)
      (`LightComponent.SetIntensity` (`self.C3Light2`) _wall_brightness)
      (`LightComponent.SetIntensity` (`self.C4Light1`) _wall_brightness)
      (`LightComponent.SetIntensity` (`self.C4Light2`) _wall_brightness))
    (:`then_1`
      (`LightComponent.SetLightColor` (`self.C1Light1`) _returnvalue_2 true)
      (`LightComponent.SetLightColor` (`self.C1Light2`) _returnvalue_2 true)
      (`LightComponent.SetLightColor` (`self.C2Light1`) _returnvalue_2 true)
      (`LightComponent.SetLightColor` (`self.C2Light2`) _returnvalue_2 true)
      (`LightComponent.SetLightColor` (`self.C3Light1`) _returnvalue_2 true)
      (`LightComponent.SetLightColor` (`self.C3Light2`) _returnvalue_2 true)
      (`LightComponent.SetLightColor` (`self.C4Light1`) _returnvalue_2 true)
      (`LightComponent.SetLightColor` (`self.C4Light2`) _returnvalue_2 true))
    (:`then_2`
      (`LightComponent.SetIntensity` (`self.CeilingLight1`) _ceiling_brightness)
      (`LightComponent.SetIntensity` (`self.CeilingLight2`) _ceiling_brightness)
      (`LightComponent.SetIntensity` (`self.CeilingLight3`) _ceiling_brightness)
      (`LightComponent.SetIntensity` (`self.CeilingLight4`) _ceiling_brightness)
      (`LightComponent.SetIntensity` (`self.CeilingLight5`) _ceiling_brightness)
      (`LightComponent.SetIntensity` (`self.CeilingLight6`) _ceiling_brightness))
    (:`then_3`
      (`LightComponent.SetLightColor` (`self.CeilingLight1`) _returnvalue true)
      (`LightComponent.SetLightColor` (`self.CeilingLight2`) _returnvalue true)
      (`LightComponent.SetLightColor` (`self.CeilingLight3`) _returnvalue true)
      (`LightComponent.SetLightColor` (`self.CeilingLight4`) _returnvalue true)
      (`LightComponent.SetLightColor` (`self.CeilingLight5`) _returnvalue true)
      (`LightComponent.SetLightColor` (`self.CeilingLight6`) _returnvalue true))))

(event `Change to Standard`
  (bind _wall_brightness (`self.wall_brightness`))
  (bind _ceiling_brightness (`self.ceiling_brightness`))
  (bind _returnvalue (`KismetMathLibrary.Conv_ColorToLinearColor` (`self.wall_color`)))
  (bind _returnvalue_2 (`KismetMathLibrary.Conv_ColorToLinearColor` (`self.ceiling_color`)))
  (`|ExecutionSequence`
    (:`then_0`
      (`LightComponent.SetIntensity` (`self.C1Light1`) _wall_brightness)
      (`LightComponent.SetIntensity` (`self.C1Light2`) _wall_brightness)
      (`LightComponent.SetIntensity` (`self.C2Light1`) _wall_brightness)
      (`LightComponent.SetIntensity` (`self.C2Light2`) _wall_brightness)
      (`LightComponent.SetIntensity` (`self.C3Light1`) _wall_brightness)
      (`LightComponent.SetIntensity` (`self.C3Light2`) _wall_brightness)
      (`LightComponent.SetIntensity` (`self.C4Light1`) _wall_brightness)
      (`LightComponent.SetIntensity` (`self.C4Light2`) _wall_brightness))
    (:`then_1`
      (`LightComponent.SetLightColor` (`self.C1Light1`) _returnvalue true)
      (`LightComponent.SetLightColor` (`self.C1Light2`) _returnvalue true)
      (`LightComponent.SetLightColor` (`self.C2Light1`) _returnvalue true)
      (`LightComponent.SetLightColor` (`self.C2Light2`) _returnvalue true)
      (`LightComponent.SetLightColor` (`self.C3Light1`) _returnvalue true)
      (`LightComponent.SetLightColor` (`self.C3Light2`) _returnvalue true)
      (`LightComponent.SetLightColor` (`self.C4Light1`) _returnvalue true)
      (`LightComponent.SetLightColor` (`self.C4Light2`) _returnvalue true))
    (:`then_2`
      (`LightComponent.SetIntensity` (`self.CeilingLight1`) _ceiling_brightness)
      (`LightComponent.SetIntensity` (`self.CeilingLight2`) _ceiling_brightness)
      (`LightComponent.SetIntensity` (`self.CeilingLight3`) _ceiling_brightness)
      (`LightComponent.SetIntensity` (`self.CeilingLight4`) _ceiling_brightness)
      (`LightComponent.SetIntensity` (`self.CeilingLight5`) _ceiling_brightness)
      (`LightComponent.SetIntensity` (`self.CeilingLight6`) _ceiling_brightness))
    (:`then_3`
      (`LightComponent.SetLightColor` (`self.CeilingLight1`) _returnvalue_2 true)
      (`LightComponent.SetLightColor` (`self.CeilingLight2`) _returnvalue_2 true)
      (`LightComponent.SetLightColor` (`self.CeilingLight3`) _returnvalue_2 true)
      (`LightComponent.SetLightColor` (`self.CeilingLight4`) _returnvalue_2 true)
      (`LightComponent.SetLightColor` (`self.CeilingLight5`) _returnvalue_2 true)
      (`LightComponent.SetLightColor` (`self.CeilingLight6`) _returnvalue_2 true))))

(fn `UserConstructionScript`
  (bind _ceiling_brightness (`self.ceiling_brightness`))
  (bind _wall_brightness (`self.wall_brightness`))
  (bind _returnvalue (`KismetMathLibrary.Conv_ColorToLinearColor` (`self.ceiling_color`)))
  (bind _returnvalue_2 (`KismetMathLibrary.Conv_ColorToLinearColor` (`self.wall_color`)))
  (`|ExecutionSequence`
    (:`then_0`
      (`LightComponent.SetIntensity` (`self.C1Light1`) _wall_brightness)
      (`LightComponent.SetIntensity` (`self.C1Light2`) _wall_brightness)
      (`LightComponent.SetIntensity` (`self.C2Light1`) _wall_brightness)
      (`LightComponent.SetIntensity` (`self.C2Light2`) _wall_brightness)
      (`LightComponent.SetIntensity` (`self.C3Light1`) _wall_brightness)
      (`LightComponent.SetIntensity` (`self.C3Light2`) _wall_brightness)
      (`LightComponent.SetIntensity` (`self.C4Light1`) _wall_brightness)
      (`LightComponent.SetIntensity` (`self.C4Light2`) _wall_brightness))
    (:`then_1`
      (`LightComponent.SetLightColor` (`self.C1Light1`) _returnvalue_2 true)
      (`LightComponent.SetLightColor` (`self.C1Light2`) _returnvalue_2 true)
      (`LightComponent.SetLightColor` (`self.C2Light1`) _returnvalue_2 true)
      (`LightComponent.SetLightColor` (`self.C2Light2`) _returnvalue_2 true)
      (`LightComponent.SetLightColor` (`self.C3Light1`) _returnvalue_2 true)
      (`LightComponent.SetLightColor` (`self.C3Light2`) _returnvalue_2 true)
      (`LightComponent.SetLightColor` (`self.C4Light1`) _returnvalue_2 true)
      (`LightComponent.SetLightColor` (`self.C4Light2`) _returnvalue_2 true))
    (:`then_2`
      (`LightComponent.SetIntensity` (`self.CeilingLight1`) _ceiling_brightness)
      (`LightComponent.SetIntensity` (`self.CeilingLight2`) _ceiling_brightness)
      (`LightComponent.SetIntensity` (`self.CeilingLight3`) _ceiling_brightness)
      (`LightComponent.SetIntensity` (`self.CeilingLight4`) _ceiling_brightness)
      (`LightComponent.SetIntensity` (`self.CeilingLight5`) _ceiling_brightness)
      (`LightComponent.SetIntensity` (`self.CeilingLight6`) _ceiling_brightness))
    (:`then_3`
      (`LightComponent.SetLightColor` (`self.CeilingLight1`) _returnvalue true)
      (`LightComponent.SetLightColor` (`self.CeilingLight2`) _returnvalue true)
      (`LightComponent.SetLightColor` (`self.CeilingLight3`) _returnvalue true)
      (`LightComponent.SetLightColor` (`self.CeilingLight4`) _returnvalue true)
      (`LightComponent.SetLightColor` (`self.CeilingLight5`) _returnvalue true)
      (`LightComponent.SetLightColor` (`self.CeilingLight6`) _returnvalue true))))