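; BP_Asteroid is a destructible asteroid that picks a random mesh, drifts by physics velocity and splits when shot down.
; Minigun and railgun bullet overlaps subtract damage and remove the bullet.
; At zero life it expires, first spawning two half-scale, half-life copies if above minimum size, adding initial life to score per copy.
; Hits between asteroids redirect velocity along the impact normal, preserving speed.
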(event `Reverse Velocity`
  (set `self.velocity` (* (`self.velocity`) -1))
  (`PrimitiveComponent.SetPhysicsLinearVelocity` (`self.AsteroidMesh`) (`self.velocity`) false "None"))

(event `self.ReceiveBeginPlay`
  (bind _scale (`self.scale`))
  (bind _asteroid_meshes (`self.asteroid_meshes`))
  (`SceneComponent.SetWorldScale3D` (`self.AsteroidMesh`) (`KismetMathLibrary.MakeVector` _scale _scale _scale))
  (set `self.initial_life` (`self.life_total`))
  (`StaticMeshComponent.SetStaticMesh` (`self.AsteroidMesh`) (`|GetArrayItem` _asteroid_meshes (`KismetMathLibrary.RandomIntegerInRange` 0 (- (`KismetArrayLibrary.Array_Length` _asteroid_meshes) 1))))
  (`PrimitiveComponent.SetPhysicsLinearVelocity` (`self.AsteroidMesh`) (`self.velocity`) false "None"))

(event `Take Damage`
  (params (damage :type "Float (double-precision)"))
  (set `self.life_total` (- (`self.life_total`) damage))
  (if (<= (`self.life_total`) 0.0)
    (`self.Break`)))

(event `Break`
  (`|ExecutionSequence`
    (:`then_0`
      (if (> (`self.scale`) (`self.split_minimum_scale`))
        (`|ExecutionSequence`
          (:`then_0`
            _)
          (:`then_1`
            _))
        (`|SpawnActorFromClass` "BP_Asteroid_C" (`self.GetTransform` self) "Undefined" "OverrideRootScale" null (/ (`self.scale`) 2.0) (`self.GetNewVelocity`) (/ (`self.initial_life`) 2.0) (`self.score_display`) null)
        (`/Game/Blueprints/BP_ScoreDisplay.Update Score` (`self.score_display`) (`KismetMathLibrary.Round` (`self.initial_life`)))))
    (:`then_1`
      (`self.SetLifeSpan` 0.01))))

(event `self.AsteroidMesh.OnComponentBeginOverlap`
  (params (OverlappedComponent :type "PrimitiveComponent Object Reference") (OtherActor :type "Actor Object Reference") (OtherComp :type "PrimitiveComponent Object Reference") (OtherBodyIndex :type Integer) (bFromSweep :type Boolean) (SweepResult :type "HitResult Structure (by ref)"))
  (bind _asbp_bullet_minigun (cast `/Game/Blueprints/BP_Bullet_Minigun` OtherActor)
    (:`then`
      (`self.Take Damage` (`/Game/Blueprints/BP_Bullet_Minigun.damage` _asbp_bullet_minigun))
      (`self.SetLifeSpan` _asbp_bullet_minigun 0.01)
      (`self.K2_SetActorLocation` _asbp_bullet_minigun (0.0 0.0 10000.0) false true))
    (:`CastFailed`
      (bind _asbp_bullet_railgun (cast `/Game/Blueprints/BP_Bullet_Railgun` OtherActor))
      (`self.Take Damage` (`/Game/Blueprints/BP_Bullet_Railgun.damage` _asbp_bullet_railgun))
      (`self.SetLifeSpan` _asbp_bullet_railgun 0.01)
      (`self.K2_SetActorLocation` _asbp_bullet_railgun (0.0 0.0 10000.0) false true))))

(event `self.AsteroidMesh.OnComponentHit`
  (params (HitComponent :type "PrimitiveComponent Object Reference") (OtherActor :type "Actor Object Reference") (OtherComp :type "PrimitiveComponent Object Reference") (NormalImpulse :type "Vector Structure") (Hit :type "HitResult Structure (by ref)"))
  (cast `/Game/Blueprints/BP_Asteroid` OtherActor)
  (set `self.velocity` (* (* (`KismetMathLibrary.Normal` (`.ImpactNormal` (`GameplayStatics.BreakHitResult` Hit))) 1) (`KismetMathLibrary.VSize` (`self.velocity`))))
  (`PrimitiveComponent.SetPhysicsLinearVelocity` (`self.AsteroidMesh`) (`self.velocity`) false "None"))

(fn `UserConstructionScript`)