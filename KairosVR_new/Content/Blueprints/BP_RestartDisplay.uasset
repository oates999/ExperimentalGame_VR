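; VR end-game restart panel that shows the final score and offers Yes to reload the current level or No to quit.
; Activate reveals it, pulls the score from BP_ScoreDisplay, plays an end-game sound and freezes time via zero global dilation; hiding also moves RestartHandle out of reach.
; Motion controller overlaps on the Yes/No volumes set and highlight the active button, falling back to the other if still overlapped.
; Releasing either trigger performs the selected action.
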(event `Key|MotionController_Left_Trigger`
  (params (Key :type "Key Structure"))
  (:`Released`
    (`self.Perform Action` :!label _label)))

(event `Get and Update Score`
  (bind _outactors (`GameplayStatics.GetAllActorsOfClass` "/Game/Blueprints/BP_ScoreDisplay.BP_ScoreDisplay_C"))
  (`self.Update Score` (`/Game/Blueprints/BP_ScoreDisplay.score` (`|GetArrayItem` _outactors))))

(event `Key|MotionController_Right_Trigger`
  (params (Key :type "Key Structure"))
  (:`Released`
    (goto _label)))

(event `self.ReceiveBeginPlay`
  (`SceneComponent.SetVisibility` (`self.RestartDisplayRoot`) false true)
  (`SceneComponent.K2_SetRelativeLocation` (`self.RestartHandle`) (0.0 0.0 1000.0) false false))

(event `Update Button Display`
  (if (`KismetStringLibrary.EqualEqual_StrStr` (`self.active_button`) "none")
    (`TextRenderComponent.SetTextRenderColor` (`self.YesText`) (`self.default_color`))
    (`TextRenderComponent.SetTextRenderColor` (`self.NoText`) (`self.default_color`))
    (elif (`KismetStringLibrary.EqualEqual_StrStr` (`self.active_button`) "Y")
      (`TextRenderComponent.SetTextRenderColor` (`self.YesText`) (`self.highlight_color`))
      (`TextRenderComponent.SetTextRenderColor` (`self.NoText`) (`self.default_color`))
      (elif (`KismetStringLibrary.EqualEqual_StrStr` (`self.active_button`) "N")
        (`TextRenderComponent.SetTextRenderColor` (`self.YesText`) (`self.default_color`))
        (`TextRenderComponent.SetTextRenderColor` (`self.NoText`) (`self.highlight_color`))))))

(event `Update Score`
  (params (score :type Integer))
  (`TextRenderComponent.K2_SetText` (`self.ScoreText`) (`KismetTextLibrary.Conv_IntToText` score)))

(event `Activate`
  (`SceneComponent.SetVisibility` (`self.RestartDisplayRoot`) true true)
  (`self.Get and Update Score`)
  (`SceneComponent.K2_SetRelativeLocation` (`self.RestartHandle`) (0.0 0.0 0.0) false false)
  (`GameplayStatics.PlaySoundAtLocation` "/Game/Assets/Sounds/endgame.endgame" (`self.K2_GetActorLocation` self) (struct) 1.0 1.0 0.0 "/Game/Assets/Sounds/NewSoundAttenuation.NewSoundAttenuation")
  (`GameplayStatics.SetGlobalTimeDilation` 0.0))

(event `Deactivate`
  (`SceneComponent.SetVisibility` (`self.RestartDisplayRoot`) false true)
  (`SceneComponent.K2_SetRelativeLocation` (`self.RestartHandle`) (0.0 0.0 1000.0) false false))

(event `Perform Action`
  (if (`KismetStringLibrary.EqualEqual_StrStr` (`self.active_button`) "Y")
    (bind _returnvalue (`GameplayStatics.GetCurrentLevelName` true))
    (`GameplayStatics.OpenLevel` (`KismetStringLibrary.Conv_StringToName` _returnvalue))
    (elif (`KismetStringLibrary.EqualEqual_StrStr` (`self.active_button`) "N")
      (`KismetSystemLibrary.QuitGame` null "Quit"))))

(event `self.YesCollision.OnComponentBeginOverlap`
  (params (OverlappedComponent :type "PrimitiveComponent Object Reference") (OtherActor :type "Actor Object Reference") (OtherComp :type "PrimitiveComponent Object Reference") (OtherBodyIndex :type Integer) (bFromSweep :type Boolean) (SweepResult :type "HitResult Structure (by ref)"))
  (cast `/Game/VirtualRealityBP/Blueprints/BP_MotionController` OtherActor)
  (set `self.yes_overlap` true)
  (set `self.active_button` "Y")
  (`self.Update Button Display` :!label _label_2))

(event `self.YesCollision.OnComponentEndOverlap`
  (params (OverlappedComponent :type "PrimitiveComponent Object Reference") (OtherActor :type "Actor Object Reference") (OtherComp :type "PrimitiveComponent Object Reference") (OtherBodyIndex :type Integer))
  (cast `/Game/VirtualRealityBP/Blueprints/BP_MotionController` OtherActor)
  (set `self.yes_overlap` false)
  (if (`self.no_overlap`)
    (set `self.active_button` "N")
    (goto _label_2)
    (else
      (set `self.active_button` "none")
      (goto _label_2))))

(event `self.NoCollision.OnComponentBeginOverlap`
  (params (OverlappedComponent :type "PrimitiveComponent Object Reference") (OtherActor :type "Actor Object Reference") (OtherComp :type "PrimitiveComponent Object Reference") (OtherBodyIndex :type Integer) (bFromSweep :type Boolean) (SweepResult :type "HitResult Structure (by ref)"))
  (cast `/Game/VirtualRealityBP/Blueprints/BP_MotionController` OtherActor)
  (set `self.no_overlap` true)
  (set `self.active_button` "N")
  (goto _label_2))

(event `self.NoCollision.OnComponentEndOverlap`
  (params (OverlappedComponent :type "PrimitiveComponent Object Reference") (OtherActor :type "Actor Object Reference") (OtherComp :type "PrimitiveComponent Object Reference") (OtherBodyIndex :type Integer))
  (cast `/Game/VirtualRealityBP/Blueprints/BP_MotionController` OtherActor)
  (set `self.no_overlap` false)
  (if (`self.yes_overlap`)
    (set `self.active_button` "Y")
    (goto _label_2)
    (else
      (set `self.active_button` "none")
      (goto _label_2))))

(fn `UserConstructionScript`)