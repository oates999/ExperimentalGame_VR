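; Railgun weapon Blueprint that fires BP_Bullet_Railgun projectiles at a target actor.
; FireAtActor enters a DoOnce that applies random spread, aims at the target and spawns a bullet with speed, damage and a range-based lifespan.
; A RateOfFire timer calls ResetFire, which reopens the DoOnce and fires again while IsFiring is set.
; A legacy debug line trace remains unconnected.
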(event `ResetFire`
  (bind _weapon_root (`self.weapon_root`))
  (bind _returnvalue (/ (`self.bullet_spread`) 2.0))
  (bind _returnvalue_2 (/ (`self.bullet_spread`) 2.0))
  (bind _returnvalue_3 (/ (`self.bullet_spread`) 2.0))
  (`|ExecutionSequence`
    (:`then_0`
      (goto _label :!via `Reset`))
    (:`then_1`
      (if (`self.is_firing`)
        (`/Engine/EditorBlueprintResources/StandardMacros.DoOnce` false :!label _label
          (:`Completed`
            (`SceneComponent.K2_SetRelativeRotation` (`self.bullet_direction`) (`KismetMathLibrary.MakeRotator` (`KismetMathLibrary.RandomFloatInRange` (* -1 _returnvalue_2) _returnvalue_2) (`KismetMathLibrary.RandomFloatInRange` (* -1 _returnvalue_3) _returnvalue_3) (`KismetMathLibrary.RandomFloatInRange` (* -1 _returnvalue) _returnvalue)) false false)
            (`SceneComponent.K2_SetWorldRotation` (`self.weapon_direction`) (`KismetMathLibrary.FindLookAtRotation` (`SceneComponent.K2_GetComponentLocation` (`self.weapon_direction`)) (`self.K2_GetActorLocation` (stale `Fire At Actor` actor))) false false)
            (`|ExecutionSequence`
              (:`then_0`
                (`KismetSystemLibrary.K2_SetTimerDelegate` (delegate `ResetFire`) (`self.rate_of_fire`)))
              (:`then_1`)
              (:`then_2`
                ;[1 1 1] Bullet Spawning
                (bind _returnvalue_4 (`|SpawnActorFromClass` "/Game/Blueprints/BP_Bullet_Railgun.BP_Bullet_Railgun_C" (`KismetMathLibrary.MakeTransform` (`SceneComponent.K2_GetComponentLocation` _weapon_root) (`SceneComponent.K2_GetComponentRotation` (`self.bullet_direction`)) (`SceneComponent.K2_GetComponentScale` _weapon_root)) "Undefined" "OverrideRootScale" null (* (`SceneComponent.GetForwardVector` (`self.bullet_direction`)) (`self.bullet_speed`)) (`self.damage`) null))
                (`self.SetLifeSpan` _returnvalue_4 (/ (`self.range`) (`self.bullet_speed`)))))))))))

(event `Fire At Actor`
  (params (actor :type "Actor Object Reference"))
  (goto _label))

(fn `UserConstructionScript`)