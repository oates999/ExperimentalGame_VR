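; BP_ShipMovementTarget is a movable target actor, named for ship movement, driven by either arrow keys or a VR motion controller.
; Key events track held keys and set one direction per axis, with the latest press winning and release reverting to the opposite held key.
; With KeyboardControls on, Tick teleports the actor in fixed, frame-rate-dependent steps along world X and Y.
; Otherwise, Tick snaps its StaticMesh to the MotionControllerPawn's left hand mesh transform.
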(event `Key|Up`
  (params (Key :type "Key Structure"))
  ;[1 1 1] Keyboard Controls
  (:`Pressed`
    (set `self.moving_up` true)
    (set `self.current_direction_vert` "Up"))
  (:`Released`
    (set `self.moving_up` false)
    (if (`self.moving_down`)
      (set `self.current_direction_vert` "Down")
      (else
        (set `self.current_direction_vert` "")))))

(event `Key|Left`
  (params (Key :type "Key Structure"))
  ;[1 1 1] Keyboard Controls
  (:`Pressed`
    (set `self.moving_left` true)
    (set `self.current_direction_hori` "Left"))
  (:`Released`
    (set `self.moving_left` false)
    (if (`self.moving_right`)
      (set `self.current_direction_hori` "Right")
      (else
        (set `self.current_direction_hori` "")))))

(event `Key|Down`
  (params (Key :type "Key Structure"))
  ;[1 1 1] Keyboard Controls
  (:`Pressed`
    (set `self.moving_down` true)
    (set `self.current_direction_vert` "Down"))
  (:`Released`
    (set `self.moving_down` false)
    (if (`self.moving_up`)
      (set `self.current_direction_vert` "Up")
      (else
        (set `self.current_direction_vert` "")))))

(event `Key|Right`
  (params (Key :type "Key Structure"))
  ;[1 1 1] Keyboard Controls
  (:`Pressed`
    (set `self.moving_right` true)
    (set `self.current_direction_hori` "Right"))
  (:`Released`
    (set `self.moving_right` false)
    (if (`self.moving_left`)
      (set `self.current_direction_hori` "Left")
      (else
        (set `self.current_direction_hori` "")))))

(event `self.ReceiveTick`
  (params (DeltaSeconds :type "Float (single-precision)"))
  (bind _current_direction_vert (`self.current_direction_vert`))
  (bind _current_direction_hori (`self.current_direction_hori`))
  (if (`self.keyboard_controls`)
    ;[1 1 1] Keyboard Controls
    (`|ExecutionSequence`
      (:`then_0`
        (if (`KismetStringLibrary.EqualEqual_StrStr` _current_direction_vert "Up")
          (`self.K2_SetActorLocation` self (+ (`self.K2_GetActorLocation` self) (1.0 0.0 0.0)) false true)
          (elif (`KismetStringLibrary.EqualEqual_StrStr` _current_direction_vert "Down")
            (`self.K2_SetActorLocation` self (+ (`self.K2_GetActorLocation` self) (-1.0 0.0 0.0)) false true))))
      (:`then_1`
        (if (`KismetStringLibrary.EqualEqual_StrStr` _current_direction_hori "Right")
          (`self.K2_SetActorLocation` self (+ (`self.K2_GetActorLocation` self) (0.0 1.0 0.0)) false true)
          (elif (`KismetStringLibrary.EqualEqual_StrStr` _current_direction_hori "Left")
            (`self.K2_SetActorLocation` self (+ (`self.K2_GetActorLocation` self) (0.0 -1.0 0.0)) false true)))))
    (else
      (bind _asmotion_controller_pawn (cast `/Game/VirtualRealityBP/Blueprints/MotionControllerPawn` (`GameplayStatics.GetPlayerPawn` 0)))
      (`SceneComponent.K2_SetWorldTransform` (`self.StaticMesh`) (`SceneComponent.K2_GetComponentToWorld` (`/Game/VirtualRealityBP/Blueprints/BP_MotionController.HandMesh` (`/Game/VirtualRealityBP/Blueprints/MotionControllerPawn.LeftController` _asmotion_controller_pawn))) false true))))

(fn `UserConstructionScript`)