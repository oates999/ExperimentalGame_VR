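; Health display Blueprint that tracks a Health counter and shows it as up to three icons.
; TakeDamage subtracts one without a lower clamp and GainHealth adds one capped at three, then both call UpdateDisplay.
; UpdateDisplay uses a branch chain to set each icon's visibility, propagated to children, hiding all for any value other than one to three.
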(event `Take Damage`
  (set `self.health` (- (`self.health`) 1))
  (`self.Update Display`))

(event `Update Display`
  (if (== (`self.health`) 3)
    (`SceneComponent.SetVisibility` (`self.HealthIcon01`) true true)
    (`SceneComponent.SetVisibility` (`self.HealthIcon02`) true true)
    (`SceneComponent.SetVisibility` (`self.HealthIcon03`) true true)
    (elif (== (`self.health`) 2)
      (`SceneComponent.SetVisibility` (`self.HealthIcon01`) true true)
      (`SceneComponent.SetVisibility` (`self.HealthIcon02`) true true)
      (`SceneComponent.SetVisibility` (`self.HealthIcon03`) false true)
      (elif (== (`self.health`) 1)
        (`SceneComponent.SetVisibility` (`self.HealthIcon01`) true true)
        (`SceneComponent.SetVisibility` (`self.HealthIcon02`) false true)
        (`SceneComponent.SetVisibility` (`self.HealthIcon03`) false true)
        (else
          (`SceneComponent.SetVisibility` (`self.HealthIcon01`) false true)
          (`SceneComponent.SetVisibility` (`self.HealthIcon02`) false true)
          (`SceneComponent.SetVisibility` (`self.HealthIcon03`) false true))))))

(event `Gain Health`
  (set `self.health` (`KismetMathLibrary.Min` (+ (`self.health`) 1) 3))
  (`self.Update Display`))

(fn `UserConstructionScript`)