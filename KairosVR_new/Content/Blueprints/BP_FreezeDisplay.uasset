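; BP_FreezeDisplay is a display Blueprint that shows a cooldown readout, apparently for a freeze ability.
; The text stays hidden from BeginPlay until UseAbility reveals it and restarts the CooldownCounter timeline.
; Each timeline update writes the Timer track's value into the text, and the text hides again when the timeline finishes.
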(event `Use Ability`
  (`SceneComponent.SetVisibility` (`self.CooldownText`) true false)
  (bind (_direction _timer) (`Timeline|Cooldown Counter` :!via `PlayFromStart`)
    (:`Update`
      (`TextRenderComponent.K2_SetText` (`self.CooldownText`) (`KismetTextLibrary.Conv_DoubleToText` _timer "HalfToEven" true 1 324 0 1)))
    (:`Finished`
      (`SceneComponent.SetVisibility` (`self.CooldownText`) false false))))

(event `self.ReceiveBeginPlay`
  (`SceneComponent.SetVisibility` (`self.CooldownText`) false false))

(fn `UserConstructionScript`)